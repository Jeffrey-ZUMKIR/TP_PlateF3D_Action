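; BP_NextLevel is a volume that completes the current level and opens the next one when the player overlaps it.
; Its overlap event filters for the player, then calls CompleteLevel, which only forwards to LoadNextLevel.
; LoadNextLevel looks up the current level's name in the LevelNames array and opens the following entry by name, with no check for the end of the list.
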(event `self.ReceiveActorBeginOverlap`
  (params (OtherActor :type "Actor Object Reference"))
  (`/Game/Blueprint/Librairies/TP_MacroLibrary.Is Player` OtherActor
    (:`Is Player`
      (`self.Complete Level`))))

(fn `Complete Level`
  (`self.Load Next Level`))

(fn `Get Current Level Index`
  (returns (`Return Value` :type Integer))
  (bind _returnvalue (`GameplayStatics.GetCurrentLevelName` true))
  (return (`KismetArrayLibrary.Array_Find` (`self.Level Names`) (`KismetStringLibrary.Conv_StringToName` _returnvalue))))

(fn `Load Next Level`
  (`GameplayStatics.OpenLevel` (`|GetArrayItem` (`self.Level Names`) (+ (`self.Get Current Level Index`) 1))))

(fn `UserConstructionScript`)
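; Tutorial trigger volume that shows on-screen hint text to the player by writing to the TextTuto variable on BP_Player.
; At BeginPlay every instance sets a welcome message with movement and camera controls, then clears it after a delay.
; When the player character overlaps the trigger, WhichTuto selects a hint on jumping, avoiding the void or collecting cards, cleared after a shorter delay.
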(event `self.ReceiveBeginPlay`
  ;[1 1 1] Explication début
  (bind _asbp_player (cast `/Game/Blueprint/Pawn/BP_Player` (`GameplayStatics.GetPlayerCharacter` 0)))
  (set `/Game/Blueprint/Pawn/BP_Player.TextTuto` "Welcome! \nPress zqsd to move around and move the mouse for the camera." _asbp_player)
  (`KismetSystemLibrary.Delay` 5.0)
  (set `/Game/Blueprint/Pawn/BP_Player.TextTuto` "" _asbp_player))

(event `self.Trigger.OnComponentBeginOverlap`
  (params (OverlappedComponent :type "PrimitiveComponent Object Reference") (OtherActor :type "Actor Object Reference") (OtherComp :type "PrimitiveComponent Object Reference") (OtherBodyIndex :type Integer) (bFromSweep :type Boolean) (SweepResult :type "HitResult Structure (by ref)"))
  (bind _returnvalue (`GameplayStatics.GetPlayerCharacter` 0))
  ;[1 1 1] Affichage Tuto
  (if (== _returnvalue OtherActor)
    (if (== (`self.WhichTuto`) 1)
      (bind _asbp_player (cast `/Game/Blueprint/Pawn/BP_Player` _returnvalue))
      (set `/Game/Blueprint/Pawn/BP_Player.TextTuto` "Use the spacebar to jump." _asbp_player)
      (`KismetSystemLibrary.Delay` 2.0 :!label _label)
      (bind _asbp_player_2 (cast `/Game/Blueprint/Pawn/BP_Player` (`GameplayStatics.GetPlayerCharacter` 0)))
      (set `/Game/Blueprint/Pawn/BP_Player.TextTuto` "" _asbp_player_2)
      (elif (== (`self.WhichTuto`) 2)
        (bind _asbp_player_3 (cast `/Game/Blueprint/Pawn/BP_Player` _returnvalue))
        (set `/Game/Blueprint/Pawn/BP_Player.TextTuto` "Do not fall in the void." _asbp_player_3)
        (goto _label)
        (elif (== (`self.WhichTuto`) 3)
          (bind _asbp_player_4 (cast `/Game/Blueprint/Pawn/BP_Player` _returnvalue))
          (set `/Game/Blueprint/Pawn/BP_Player.TextTuto` "Collect all the cards for each suits." _asbp_player_4)
          (goto _label))))))

(fn `UserConstructionScript`)
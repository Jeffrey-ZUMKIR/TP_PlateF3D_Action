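; BP_Carte is a collectable playing card that adds to the player's card count and score on overlap, then destroys itself.
; On BeginPlay it pushes suit, value and back design into front and back widget components.
; The Card_Floating timeline animates the card's relative height and yaw.
; An unconnected branch that would increment and print a card count on BP_GameInstance never runs.
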(event `self.ReceiveBeginPlay`
  (bind _card (`self.Card`))
  (bind _asmy_card_face (cast `/Game/Blueprint/Collectables/Widget/My_Card_Face` (`WidgetComponent.GetUserWidgetObject` (`self.My card widget`))))
  (set `/Game/Blueprint/Collectables/Widget/My_Card_Face.FinalCardSuit` (`self.Suit`) _asmy_card_face)
  (`TextBlock.SetText` (`/Game/Blueprint/Collectables/Widget/My_Card_Face.Cardvalue` _asmy_card_face) (`self.Value`))
  (bind _asmy_card_back (cast `/Game/Blueprint/Collectables/Widget/My_Card_Back` (`WidgetComponent.GetUserWidgetObject` (`self.My card back`))))
  (set `/Game/Blueprint/Collectables/Widget/My_Card_Back.FinalDos` "/Game/Blueprint/Collectables/Image/Dos.Dos" _asmy_card_back)
  ;[1 1 1] Animation Carte
  (bind (_direction _cardheightlocation _cardrotation) (`Timeline|Card_Floating` :!via `PlayFromStart`)
    (:`Update`
      (`SceneComponent.K2_SetRelativeLocation` _card (`KismetMathLibrary.VLerp` (`self.InitialLocation`) (`self.DestinationLocation`) _cardheightlocation) false false)
      (`SceneComponent.K2_SetRelativeRotation` _card (`KismetMathLibrary.MakeRotator` 0.0 0.0 (* 10 _cardrotation)) false false))))

(event `self.ReceiveActorBeginOverlap`
  (params (OtherActor :type "Actor Object Reference"))
  ;[1 1 1] Collecte
  (`/Game/Blueprint/Librairies/TP_MacroLibrary.Is Player` OtherActor
    (:`Is Player`
      (`self.K2_DestroyActor`)
      (bind _asbp_player (cast `/Game/Blueprint/Pawn/BP_Player` (`GameplayStatics.GetPlayerCharacter` 0)))
      (set `/Game/Blueprint/Pawn/BP_Player.Card` (+ (`/Game/Blueprint/Pawn/BP_Player.Card` _asbp_player) 1) _asbp_player)
      (set `/Game/Blueprint/Pawn/BP_Player.Score` (+ (`/Game/Blueprint/Pawn/BP_Player.Score` _asbp_player) (`self.ScoreValue`)) _asbp_player))))

(fn `UserConstructionScript`)